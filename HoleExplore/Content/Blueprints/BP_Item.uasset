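; BP_Item is a world item that BP_PlayerCharacter can pick up and drop.
; Overlapping its RenderComponent registers it as the character's OverlapItem and immediately calls Pick, while ending overlap clears that reference.
; OnPickup hides it, disables collision and clears overlapping characters' references, while OnDrop restores it at a given position.
; A RepNotify on the pickup flag mirrors visibility and collision.
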(event `self.ReceiveBeginPlay`)

(event `self.ReceiveActorBeginOverlap`
  (params (OtherActor :type "Actor Object Reference")))

(event `self.ReceiveTick`
  (params (DeltaSeconds :type "Float (single-precision)")))

(event `self.RenderComponent.OnComponentBeginOverlap`
  (params (OtherActor :type "Actor Object Reference") (OtherComp :type "PrimitiveComponent Object Reference") (OtherBodyIndex :type Integer) (bFromSweep :type Boolean) (SweepResult :type "HitResult Structure (by ref)"))
  (bind _asbp_player_character (cast `/Game/Blueprints/BP_PlayerCharacter` OtherActor))
  (set `/Game/Blueprints/BP_PlayerCharacter.OverlapItem` self _asbp_player_character)
  (`/Game/Blueprints/BP_PlayerCharacter.Pick` _asbp_player_character))

(event `self.RenderComponent.OnComponentEndOverlap`
  (params (OtherActor :type "Actor Object Reference") (OtherComp :type "PrimitiveComponent Object Reference") (OtherBodyIndex :type Integer))
  (bind _asbp_player_character (cast `/Game/Blueprints/BP_PlayerCharacter` OtherActor))
  (set `/Game/Blueprints/BP_PlayerCharacter.OverlapItem` null _asbp_player_character))

(fn `OnDrop`
  (params (Position :type "Vector Structure"))
  (set `self.bPickuped` false)
  (`self.SetActorEnableCollision` true)
  (`self.SetActorHiddenInGame` false)
  (`self.K2_SetActorLocation` Position))

(fn `OnPickup`
  (set `self.bPickuped` true)
  (`self.SetActorHiddenInGame` true)
  (`self.SetActorEnableCollision` false)
  (for _array_element (`PrimitiveComponent.GetOverlappingActors` (`self.RenderComponent`) "/Game/Blueprints/BP_PlayerCharacter.BP_PlayerCharacter_C")
    (bind _asbp_player_character (cast `/Game/Blueprints/BP_PlayerCharacter` _array_element))
    (set `/Game/Blueprints/BP_PlayerCharacter.OverlapItem` null _asbp_player_character)))

(fn `OnRep_bPickuped`
  (bind _bpickuped (`self.bPickuped`))
  (`self.SetActorEnableCollision` (not _bpickuped))
  (`self.SetActorHiddenInGame` _bpickuped))

(fn `UserConstructionScript`)