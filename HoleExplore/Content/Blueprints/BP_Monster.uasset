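; Paper2D monster that wanders at random, damages the player on contact and dies from any single hit.
; Tick runs SelectAI, which makes a swept random step in the X/Z plane, then waits on a random timer.
; Box overlap applies damage to BP_PlayerCharacter.
; When damaged, it disables collision and tick, shows DeadFlipbook, fades out by timeline, then destroys itself, removing itself from BelongRoom via OnDestroyed.
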(event `OnTakeAnyDamage_Event_0` :!signature `self.OnTakeAnyDamage`
  (params (Damage :type "Float (double-precision)") (DamageType :type "DamageType Object Reference") (InstigatedBy :type "Controller Object Reference") (DamageCauser :type "Actor Object Reference"))
  (bind _deadflipbook (`self.DeadFlipbook`))
  (`|ExecutionSequence`
    (:`then_1`
      (`self.SetActorEnableCollision` false))
    (:`then_2`
      (`self.SetActorTickEnabled` false))
    (:`then_3`
      (`/Engine/EditorBlueprintResources/StandardMacros.IsValid` _deadflipbook
        (:`Is Valid`
          (`PaperFlipbookComponent.SetFlipbook` (`self.PaperFlipbook`) _deadflipbook))))
    (:`then_4`
      (bind (_direction _alpha) (`Timeline|Dead` :!via `PlayFromStart`)
        (:`Update`
          (`PaperFlipbookComponent.SetSpriteColor` (`self.PaperFlipbook`) (`KismetMathLibrary.MakeColor` 1.0 1.0 1.0 _alpha)))
        (:`Finished`
          (`self.K2_DestroyActor`))))))

(event `self.ReceiveBeginPlay`
  (`|ExecutionSequence`
    (:`then_0`
      (add `self.OnTakeAnyDamage` (delegate `OnTakeAnyDamage_Event_0`)))
    (:`then_1`
      (add `self.OnDestroyed` (delegate `OnDestroyed_Event_0`)))))

(event `self.ReceiveActorBeginOverlap`
  (params (OtherActor :type "Actor Object Reference")))

(event `OnDestroyed_Event_0`
  (`/Game/Blueprints/BP_Room.RemoveAMonster` (`self.BelongRoom`) self))

(event `self.ReceiveTick`
  (params (DeltaSeconds :type "Float (single-precision)"))
  (`self.SelectAI`))

(event `self.Box.OnComponentBeginOverlap`
  (params (OtherActor :type "Actor Object Reference") (OtherComp :type "PrimitiveComponent Object Reference") (OtherBodyIndex :type Integer) (bFromSweep :type Boolean) (SweepResult :type "HitResult Structure (by ref)"))
  (bind _asbp_player_character (cast `/Game/Blueprints/BP_PlayerCharacter` OtherActor))
  (`GameplayStatics.ApplyDamage` _asbp_player_character 1.0 null self))

(event `SelectAI`
  (if (not (`self.bActionExecuting`))
    (`self.K2_AddActorLocalOffset` (* (`KismetMathLibrary.MakeVector` (select `int` (`KismetMathLibrary.RandomIntegerInRange` 0 2) :`0` -1.0 :`1` 0.0 :`2` 1.0 :!type "Float (single-precision)") 0.0 (select `int` (`KismetMathLibrary.RandomIntegerInRange` 0 2) :`0` -1.0 :`1` 0.0 :`2` 1.0 :!type "Float (single-precision)")) (`self.MoveAmount`)) true)
    (set `self.bActionExecuting` true)
    (`KismetSystemLibrary.K2_SetTimerDelegate` (delegate `CustomEvent_0`) (`KismetMathLibrary.RandomFloatInRange` 0.2 0.9))))

(event `CustomEvent_0`
  (set `self.bActionExecuting` false))

(fn `UserConstructionScript`)