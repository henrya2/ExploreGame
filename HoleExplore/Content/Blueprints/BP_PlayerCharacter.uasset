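; Paper2D player character that walks on the X/Z plane, fires projectiles, uses doors and carries items.
; Movement updates derive four-way flipbook animation and facing from velocity, and that facing aims projectiles, which a timer rate-limits.
; Use calls the current DoorSwitch to teleport the player, while Pick stores the overlapped item in an eight-slot array with drop, completeness and clear helpers.
; Any damage immediately opens the MainMenu level.
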(event `OnTakeAnyDamage_Event_0` :!signature `self.OnTakeAnyDamage`
  (params (Damage :type "Float (double-precision)") (DamageType :type "DamageType Object Reference") (InstigatedBy :type "Controller Object Reference") (DamageCauser :type "Actor Object Reference"))
  (`GameplayStatics.OpenLevel` "MainMenu" false))

(event `self.ReceiveBeginPlay`
  (`|ExecutionSequence`
    (:`then_0`
      (add `self.OnCharacterMovementUpdated` (delegate `OnCharacterMovementUpdated_Event_0`)))
    (:`then_1`
      (add `self.OnTakeAnyDamage` (delegate `OnTakeAnyDamage_Event_0`)))))

(event `OnCharacterMovementUpdated_Event_0` :!signature `self.OnCharacterMovementUpdated`
  (params (DeltaSeconds :type "Float (double-precision)") (OldLocation :type "Vector Structure") (OldVelocity :type "Vector Structure"))
  (bind _velocity (`MovementComponent.Velocity` (`self.CharacterMovement`)))
  (bind _x (.x _velocity))
  (if (== (`KismetMathLibrary.VSize` _velocity) 0.0)
    (`PaperFlipbookComponent.Stop` (`self.Sprite`))
    (else
      (if (== _x 0.0)
        (if (> (.z _velocity) 0.0)
          (set `self.AnimState` "NewEnumerator2")
          (else
            (set `self.AnimState` "NewEnumerator3")))
        (elif (> _x 0.0)
          (set `self.AnimState` "NewEnumerator0")
          (else
            (set `self.AnimState` "NewEnumerator1"))))
      (`self.UpdateAnim`)
      (`PaperFlipbookComponent.Play` (`self.Sprite`))
      (set `self.Direction` (select `/Game/Blueprints/Enums/E_PlayerAnimState` (`self.AnimState`) :`NewEnumerator0` "NewEnumerator4" :`NewEnumerator1` "NewEnumerator5" :`NewEnumerator2` "NewEnumerator6" :`NewEnumerator3` "NewEnumerator7" :!type "/Game/Blueprints/Enums/E_Direction Enum")))))

(event `self.ReceiveActorBeginOverlap`
  (params (OtherActor :type "Actor Object Reference")))

(event `self.ReceiveTick`
  (params (DeltaSeconds :type "Float (single-precision)")))

(event `Key|One`)

(event `InputAxis|MoveRight`
  (params (AxisValue :type "Float (single-precision)"))
  (`self.AddMovementInput` (1.0 0.0 0.0) AxisValue))

(event `Key|Two`)

(event `Key|Three`)

(event `InputAxis|MoveUp`
  (params (AxisValue :type "Float (single-precision)"))
  (`self.AddMovementInput` (0.0 0.0 1.0) AxisValue))

(event `Key|Four`)

(event `Use`
  (bind _doorswitch (`self.DoorSwitch`))
  (`/Engine/EditorBlueprintResources/StandardMacros.IsValid` _doorswitch
    (:`Is Valid`
      (`/Game/Blueprints/BP_DoorSwitch.TeleportTo` _doorswitch self)
      (`KismetSystemLibrary.PrintString` "EnterDoor"))))

(event `InputAction|Fire`
  (:`Pressed`
    (if (`self.bCanFire`)
      (`self.FireProjectile`)
      (`|ExecutionSequence`
        (:`then_0`
          (set `self.bCanFire` false))
        (:`then_1`
          (`KismetSystemLibrary.K2_SetTimerDelegate` (delegate `CustomEvent_0`) (`self.FireInterval`)))))))

(event `FireProjectile`
  (`|SpawnActorFromClass` "/Game/Blueprints/BP_Projectile.BP_Projectile_C" (`KismetMathLibrary.MakeTransform` (`self.K2_GetActorLocation`) (select `/Game/Blueprints/Enums/E_Direction` (`self.Direction`) :`NewEnumerator5` (struct :`Yaw` 180.0) :`NewEnumerator6` (struct :`Pitch` 90.0) :`NewEnumerator7` (struct :`Pitch` -90.0) :!type "Rotator Structure")) true self self))

(event `CustomEvent_0`
  (set `self.bCanFire` true))

(event `OnFinishedPlaying_Event_0`
  (`self.Use`))

(event `Pick`
  (bind _overlapitem (`self.OverlapItem`))
  (`/Engine/EditorBlueprintResources/StandardMacros.IsValid` _overlapitem
    (:`Is Valid`
      (`self.AddItem` _overlapitem))))

(event `InputAction|Use`
  (:`Pressed`
    (`self.Use`)))

(event `AddItem`
  (params (Item :type "/Game/Blueprints/BP_Item Object Reference"))
  (bind _success (`self.PutItemIn` Item))
  (if _success
    (`/Game/Blueprints/BP_Item.OnPickup` Item)))

(event `DropItem`
  (params (Index :type Integer))
  (bind _item (`KismetArrayLibrary.Array_Get` (`self.Items`) Index))
  (`/Engine/EditorBlueprintResources/StandardMacros.IsValid` _item
    (:`Is Valid`
      (`/Game/Blueprints/BP_Item.OnDrop` _item (`self.K2_GetActorLocation`))
      (`KismetArrayLibrary.Array_Set` (`self.Items`) Index null))))

(event `UpdateAnim`
  (`PaperFlipbookComponent.SetFlipbook` (`self.Sprite`) (select `/Game/Blueprints/Enums/E_PlayerAnimState` (`self.AnimState`) :`NewEnumerator0` "/Game/Flipbooks/Characters/GirlAnimWalkRight.GirlAnimWalkRight" :`NewEnumerator1` "/Game/Flipbooks/Characters/GirlAnimWalkLeft.GirlAnimWalkLeft" :`NewEnumerator2` "/Game/Flipbooks/Characters/GirlAnimWalkUp_Flipbook.GirlAnimWalkUp_Flipbook" :`NewEnumerator3` "/Game/Flipbooks/Characters/GirlAnimWalkDown_Flipbook.GirlAnimWalkDown_Flipbook" :!type "PaperFlipbook Object Reference")))

(fn `ClearItems`
  (bind _items (`self.Items`))
  (for _array_element _items
    (`self.K2_DestroyActor` _array_element))
  (`KismetArrayLibrary.Array_Clear` _items))

(fn `IsItemCollectionComplete`
  (returns (bComplete :type Boolean))
  (set `self.bCompleteCollected` true)
  (for _array_element (`self.Items`)
    (`/Engine/EditorBlueprintResources/StandardMacros.IsValid` _array_element
      (:`Is Not Valid`
        (set `self.bCompleteCollected` false)
        (break))))
  (return (`self.bCompleteCollected`)))

(fn `PutItemIn`
  (params (Item :type "/Game/Blueprints/BP_Item Object Reference"))
  (returns (Success :type Boolean))
  (bind _items (`self.Items`))
  (set `self.bFindEmptSlot` false)
  (for _index (range (`KismetArrayLibrary.Array_Length` _items))
    (`/Engine/EditorBlueprintResources/StandardMacros.IsValid` (`KismetArrayLibrary.Array_Get` _items _index)
      (:`Is Not Valid`
        (`KismetArrayLibrary.Array_Set` _items _index Item)
        (set `self.bFindEmptSlot` true)
        (break))))
  (return (`self.bFindEmptSlot`)))

(fn `UserConstructionScript`
  (`KismetArrayLibrary.Array_Resize` (`self.Items`) 8))