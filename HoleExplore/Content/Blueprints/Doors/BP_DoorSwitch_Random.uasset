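; BP_DoorSwitch_Random is a door switch that teleports the player to a random door once its own room is clear.
; Its Teleportto event clears the room's monsters, then uses RandomManager to pick a door, spawning monsters in that door's room before moving the player there.
; A player with a complete item collection goes to the manager's UltimateDoor instead and has their items cleared.
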(event `self.ReceiveBeginPlay`
  (`parent.ReceiveBeginPlay`))

(event `self.ReceiveActorBeginOverlap`
  (params (OtherActor :type "Actor Object Reference")))

(event `self.ReceiveTick`
  (params (DeltaSeconds :type "Float (single-precision)")))

(event `self.TeleportTo`
  (params (Player :type "/Game/Blueprints/BP_PlayerCharacter Object Reference"))
  (bind _randommanager (`self.RandomManager`))
  (bind _result (`/Game/Blueprints/BP_Room.IsRoomClear` (`self.BelongRoom`)))
  (if _result
    (`/Game/Blueprints/BP_Room.ClearMonsters` (`self.BelongRoom`))
    (`/Engine/EditorBlueprintResources/StandardMacros.IsValid` _randommanager
      (:`Is Valid`
        (bind _bcomplete (`/Game/Blueprints/BP_PlayerCharacter.IsItemCollectionComplete` Player))
        (if _bcomplete
          (`self.K2_TeleportTo` :`self` Player :`DestLocation` (`self.K2_GetActorLocation` (`/Game/Blueprints/BP_RandomGameManager.UltimateDoor` _randommanager)))
          (`/Game/Blueprints/BP_PlayerCharacter.ClearItems` Player)
          (else
            (bind _door (`/Game/Blueprints/BP_RandomGameManager.GetRandomDoor` _randommanager null))
            (`/Game/Blueprints/BP_Room.SpawnMonsters` (`/Game/Blueprints/BP_DoorSwitch.BelongRoom` _door) (`self.K2_GetActorLocation` _door))
            (`self.K2_TeleportTo` :`self` Player :`DestLocation` (`self.K2_GetActorLocation` _door))))))))

(fn `UserConstructionScript`
  (`parent.UserConstructionScript`))