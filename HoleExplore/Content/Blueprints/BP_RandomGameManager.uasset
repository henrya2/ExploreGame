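; Game manager actor that coordinates the random door switches and randomizes which items appear in their rooms.
; On BeginPlay it registers itself with every BP_DoorSwitch_Random, storing the "Ultimate"-tagged door apart from the random door pool.
; It then shuffles the item classes and spawns one per pooled door at a random position in that door's room, assigning it as the RoomItem.
; GetRandomDoor returns a random pooled door other than the one passed in.
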(event `self.ReceiveBeginPlay`
  (`|ExecutionSequence`
    (:`then_0`
      (bind _outactors (`GameplayStatics.GetAllActorsOfClass` "/Game/Blueprints/Doors/BP_DoorSwitch_Random.BP_DoorSwitch_Random_C"))
      (for _array_element _outactors
        (set `/Game/Blueprints/Doors/BP_DoorSwitch_Random.RandomManager` self _array_element)
        (if (`self.ActorHasTag` _array_element "Ultimate")
          (set `self.UltimateDoor` _array_element)
          (else
            (`KismetArrayLibrary.Array_Add` (`self.RandomDoors`) _array_element)))))
    (:`then_1`
      (`KismetArrayLibrary.Array_Shuffle` (`self.SpawnItemClasses`))
      (for (_array_element_2 _array_index) (`self.SpawnItemClasses`)
        (if (< _array_index (`KismetArrayLibrary.Array_Length` (`self.RandomDoors`)))
          (bind _belongroom (`/Game/Blueprints/BP_DoorSwitch.BelongRoom` (`KismetArrayLibrary.Array_Get` (`self.RandomDoors`) _array_index)))
          (bind _position (`/Game/Blueprints/BP_Room.GetRandomItemPosition` _belongroom))
          (bind _returnvalue (`|SpawnActorFromClass` _array_element_2 (`KismetMathLibrary.MakeTransform` (`KismetMathLibrary.MakeVector` (.x _position) 1.0 (.z _position)))))
          (set `/Game/Blueprints/BP_Room.RoomItem` _returnvalue _belongroom))))))

(event `self.ReceiveActorBeginOverlap`
  (params (OtherActor :type "Actor Object Reference")))

(event `self.ReceiveTick`
  (params (DeltaSeconds :type "Float (single-precision)")))

(fn `GetRandomDoor`
  (params (SelfDoor :type "/Game/Blueprints/Doors/BP_DoorSwitch_Random Object Reference"))
  (returns (Door :type "/Game/Blueprints/Doors/BP_DoorSwitch_Random Object Reference"))
  (bind _output_get (set `self.TmpDoorArray` (`self.RandomDoors`)))
  (`KismetArrayLibrary.Array_RemoveItem` _output_get SelfDoor)
  (return (`KismetArrayLibrary.Array_Get` (`self.TmpDoorArray`) (`KismetMathLibrary.RandomIntegerInRange` 0 (- (`KismetArrayLibrary.Array_Length` _output_get) 1)))))

(fn `UserConstructionScript`)