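; BP_Room is a room actor that spawns, tracks and clears the monsters belonging to it.
; SpawnMonsters creates one to three random-class monsters at random XZ points from four box areas on a fixed Y plane, ignoring DoorPoint's value.
; AddMonster registers each and sets its BelongRoom, while RemoveAMonster and ClearMonsters empty the list.
; IsRoomClear is true only for an empty list, and GetRandomItemPosition picks a point within SpawnArea.
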(event EventBeginPlay)

(fn ConstructionScript)

(fn AddMonster
  (params (Monster :type BP%20Monster%20Object%20Reference))
  (Utilities|Array|Add (Variables|Default|GetMonsters) Monster)
  (Variables|/Game/Blueprints/BP_Monster.BP_Monster_C|SetBelongRoom Monster self))

(fn SpawnMonsters
  (params (DoorPoint :type Vector))
  (CallFunction|GetSpawnMonsterAreas)
  (for _index (range 1 (Math|Random|RandomIntegerinRange 1 3))
    (bind _monster (CallFunction|SpawnOneMonster DoorPoint))
    (CallFunction|AddMonster _monster)))

(fn GetRandomItemPosition
  (bind _spawnarea (Variables|Default|GetSpawnArea))
  (bind _boxextent (Variables|/Script/Engine.BoxComponent|GetBoxExtent _spawnarea))
  (return (Math|Random|RandomPointinBoundingBox (Transformation|GetWorldLocation _spawnarea) (Math|Vector|MakeVector (.x _boxextent) 0.0 (.z _boxextent)))))

(fn GetSpawnMonsterAreas
  (bind _spawnmonsterareas (Variables|Default|GetSpawnMonsterAreas))
  (Utilities|Array|Clear (Variables|Default|GetSpawnMonsterAreas))
  (Utilities|FlowControl|Sequence
    (:then_0
      (Utilities|Array|Add _spawnmonsterareas (Variables|Default|GetSpawnMonster1)))
    (:then_1
      (Utilities|Array|Add _spawnmonsterareas (Variables|Default|GetSpawnMonster2)))
    (:then_2
      (Utilities|Array|Add _spawnmonsterareas (Variables|Default|GetSpawnMonster3)))
    (:then_3
      (Utilities|Array|Add _spawnmonsterareas (Variables|Default|GetSpawnMonster4)))
    (:then_4
      (return (Variables|Default|GetSpawnMonsterAreas)))))

(fn SpawnOneMonster
  (params (DoorPoint :type Vector))
  (bind _spawnmonsterareas (Variables|Default|GetSpawnMonsterAreas))
  (bind _monsterclasses (Variables|Default|GetMonsterClasses))
  (bind _returnvalue (Utilities|Array|Length _spawnmonsterareas))
  (bind _returnvalue_2 (- _returnvalue 1))
  (bind _returnvalue_3 (Math|Random|RandomIntegerinRange 0 _returnvalue_2))
  (bind _item (Utilities|Array|Get(acopy) _spawnmonsterareas _returnvalue_3))
  (bind _returnvalue_4 (Transformation|GetWorldLocation _item))
  (bind _boxextent (Variables|/Script/Engine.BoxComponent|GetBoxExtent _item))
  (bind (_x _y _z) (Math|Vector|BreakVector _boxextent))
  (bind _returnvalue_5 (Math|Vector|MakeVector _x 0.0 _z))
  (bind _returnvalue_6 (Math|Random|RandomPointinBoundingBox _returnvalue_4 _returnvalue_5))
  (bind (_x_2 _y_2 _z_2) (Math|Vector|BreakVector _returnvalue_6))
  (bind _returnvalue_7 (Game|SpawnActorfromClass (Utilities|Array|Get(acopy) _monsterclasses (Math|Random|RandomIntegerinRange 0 (- (Utilities|Array|Length _monsterclasses) 1))) (Math|Transform|MakeTransform (Math|Vector|MakeVector _x_2 1.0 _z_2)) false 0 0))
  (return _returnvalue_7))

(fn ClearMonsters
  (bind _monsters (Variables|Default|GetMonsters))
  (for _array_element _monsters
    (Utilities|IsValid _array_element
      (:Is%20Valid
        (Actor|DestroyActor _array_element))))
  (Utilities|Array|Clear _monsters))

(fn IsRoomClear
  (bind _output_get (LocalVariables|SetbTmpResult (== (Utilities|Array|Length (Variables|Default|GetMonsters)) 0)))
  (if _output_get
    _
    (else
      (bind _array_element (Utilities|Array|ForEachLoopwithBreak (Variables|Default|GetMonsters) :!label _label)
        (:LoopBody
          (Utilities|IsValid _array_element
            (:Is%20Not%20Valid
              (LocalVariables|SetbTmpResult false)
              (goto _label Break))))
        (:Completed
          _))))
  (return (LocalVariables|GetbTmpResult)))

(fn RemoveAMonster
  (params (Monster :type BP%20Monster%20Object%20Reference))
  (Utilities|Array|RemoveItem (Variables|Default|GetMonsters) Monster))