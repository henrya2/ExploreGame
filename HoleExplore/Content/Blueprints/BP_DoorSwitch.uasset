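; BP_DoorSwitch is a door that can teleport a player to the location of a linked TeleportActor.
; On the authority only, its DoorTrigger overlap registers the door as the DoorSwitch on an entering BP_PlayerCharacter and clears it on exit.
; Its TeleportTo event moves the given player there with zero rotation, and BeginPlay stops the render component's playback and disables looping.
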(event `self.ReceiveBeginPlay`
  (bind _rendercomponent (`self.RenderComponent`))
  (`PaperFlipbookComponent.Stop` _rendercomponent)
  (`PaperFlipbookComponent.SetLooping` _rendercomponent false))

(event `self.ReceiveActorBeginOverlap`
  (params (OtherActor :type "Actor Object Reference")))

(event `self.ReceiveTick`
  (params (DeltaSeconds :type "Float (single-precision)")))

(event `self.DoorTrigger.OnComponentBeginOverlap`
  (params (OtherActor :type "Actor Object Reference") (OtherComp :type "PrimitiveComponent Object Reference") (OtherBodyIndex :type Integer) (bFromSweep :type Boolean) (SweepResult :type "HitResult Structure (by ref)"))
  (`/Engine/EditorBlueprintResources/ActorMacros.Switch Has Authority`
    (:`Authority`
      (bind _asbp_player_character (cast `/Game/Blueprints/BP_PlayerCharacter` OtherActor))
      (set `/Game/Blueprints/BP_PlayerCharacter.DoorSwitch` self _asbp_player_character))))

(event `self.DoorTrigger.OnComponentEndOverlap`
  (params (OtherActor :type "Actor Object Reference") (OtherComp :type "PrimitiveComponent Object Reference") (OtherBodyIndex :type Integer))
  (`/Engine/EditorBlueprintResources/ActorMacros.Switch Has Authority`
    (:`Authority`
      (bind _asbp_player_character (cast `/Game/Blueprints/BP_PlayerCharacter` OtherActor))
      (set `/Game/Blueprints/BP_PlayerCharacter.DoorSwitch` null _asbp_player_character))))

(event `TeleportTo`
  (params (Player :type "/Game/Blueprints/BP_PlayerCharacter Object Reference"))
  (`self.K2_TeleportTo` :`self` Player :`DestLocation` (`self.K2_GetActorLocation` (`self.TeleportActor`))))

(fn `UserConstructionScript`)